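; Base character Blueprint for stance-based melee combat, handling hit, block breach, parry, stance switch and death reactions.
; BeginPlay binds events from the ACHealth and ACCombatSystem components; handlers play montages and adjust character state, walk speed and time dilation.
; Left or right pose selects montages and sections, with randomized heavy-hit and death variants.
; Death freezes the mesh in a matching pose and disables collision, with empty widget hooks.
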(event Custom|Hit%20Animation
  (params (Attack%20Type :type E_AttackType%20Enum :default "NewEnumerator1"))
  (bind (_damage_monatge _section) (CallFunction|GetTakeHeavyDamageAnimation))
  (if (Utilities|Enum|Equal(Enum) Attack%20Type "NewEnumerator4")
    (Animation|Montage|PlayMontage (Variables|Character|GetMesh) _damage_monatge 1.25 0.0 _section)
    (else
      (Animation|StopAnimMontage 0)
      (Variables|Default|SetCharacter%20State "NewEnumerator1"))))

(event Custom|Death%20Animation
  (Variables|Death|SetbDead true)
  (Animation|Montage|PlayMontage (Variables|Character|GetMesh) "/Game/Player/Animation/Death/AM_Death.AM_Death" 1.0 0.0 (CallFunction|GetDeathAnimation (Variables|Default|GetCharacter%20Pose))
    (:then
      (CallFunction|ControlWidgetOff))
    (:OnBlendOut
      (CallFunction|DeathProcessing)
      (CallFunction|DeathMenuWidget))))

(event Custom|Breach
  (bind _section (CallFunction|GetBreachAnimation))
  (Animation|Montage|PlayMontage (Variables|Character|GetMesh) "/Game/Player/Animation/Block/AM_Breach.AM_Breach" 1.0 0.0 _section
    (:then
      (Variables|Default|SetCharacter%20State "NewEnumerator1"))
    (:OnBlendOut
      (Variables|/Script/Engine.CharacterMovementComponent|SetMaxWalkSpeed (Variables|Character|GetCharacterMovement) 5e+02)
      (Variables|/Game/Blueprints/AC_CombatSystem.AC_CombatSystem_C|SetbKnocked (Variables|Default|GetAC_CombatSystem) false))))

(event Custom|Damage%20Slow%20Out
  (bind _ac_combatsystem (Variables|Default|GetAC_CombatSystem))
  (bind _charactermovement (Variables|Character|GetCharacterMovement))
  (Utilities|FlowControl|Delay (Variables|Damage|GetSlow%20Duration))
  (if (Utilities|Enum|Equal(Enum) (Variables|Default|GetCharacter%20State) "NewEnumerator3")
    (Variables|/Script/Engine.CharacterMovementComponent|SetMaxWalkSpeed _charactermovement (Variables|/Game/Blueprints/AC_CombatSystem.AC_CombatSystem_C|GetBlock%20Move%20Speed _ac_combatsystem))
    (else
      (Variables|/Script/Engine.CharacterMovementComponent|SetMaxWalkSpeed _charactermovement (Variables|/Game/Blueprints/AC_CombatSystem.AC_CombatSystem_C|GetDefault%20Move%20Speed _ac_combatsystem))))
  (Variables|Damage|SetbTakingDamage false))

(event Custom|Parry%20Out
  (Utilities|FlowControl|Delay (Variables|Block|GetParry%20Dilation%20Duration))
  (Utilities|Time|SetGlobalTimeDilation 1.0))

(event Custom|Parry
  (params (Instigator :type BP%20Base%20Character%20Object%20Reference))
  (Animation|StopAnimMontage 0)
  (Animation|Montage|PlayMontage (Variables|Character|GetMesh) "/Game/Player/Animation/Parry/AM_Parry.AM_Parry"
    (:then
      (Animation|StopAnimMontage Instigator 0)
      (Variables|Default|SetCharacter%20State "NewEnumerator1")
      (Variables|BP_BaseCharacter_C|SetCharacter%20State Instigator "NewEnumerator1")
      (Animation|Montage|PlayMontage (Variables|/Script/Engine.Character|GetMesh Instigator) "/Game/Player/Animation/TakeDamage/AM_HitHeavy_LP.AM_HitHeavy_LP" 1.0 0.0 (.Section (CallFunction|GetTakeHeavyDamageAnimation))))))

(event Custom|Switch%20Pose
  (bind _mesh (Variables|Character|GetMesh))
  (bind _charactermovement (Variables|Character|GetCharacterMovement))
  (if (Utilities|Enum|Equal(Enum) (Variables|Default|GetCharacter%20Pose) "NewEnumerator1")
    (Variables|Default|SetCharacter%20Pose "NewEnumerator2")
    (Animation|Montage|PlayMontage _mesh "/Game/Player/Animation/LocomotionLP/AM_LP2RP.AM_LP2RP" 1.5
      (:then
        (Variables|/Script/Engine.CharacterMovementComponent|SetMaxWalkSpeed _charactermovement 0.0 :!label _label))
      (:OnBlendOut
        (Variables|/Script/Engine.CharacterMovementComponent|SetMaxWalkSpeed _charactermovement 5e+02 :!label _label_2)))
    (else
      (Variables|Default|SetCharacter%20Pose "NewEnumerator1")
      (Animation|Montage|PlayMontage _mesh "/Game/Player/Animation/LocomotionRP/AM_RP2LP.AM_RP2LP" 1.5
        (:then
          (goto _label))
        (:OnBlendOut
          (goto _label_2))))))

(event EventBeginPlay
  (CallFunction|BindEvents))

(fn ConstructionScript)

(fn GetTakeHeavyDamageAnimation
  (switch Utilities|FlowControl|Switch|SwitchonE_CharacterState (Variables|Default|GetCharacter%20State)
    (:NewEnumerator1
      _)
    (:NewEnumerator4
      _))
  (switch Utilities|FlowControl|Switch|SwitchonE_CharacterPose (Variables|Default|GetCharacter%20Pose)
    (:NewEnumerator1
      (LocalVariables|SetDamage%20Animation "/Game/Player/Animation/TakeDamage/AM_HitHeavy_LP.AM_HitHeavy_LP"))
    (:NewEnumerator2
      (LocalVariables|SetDamage%20Animation "/Game/Player/Animation/TakeDamage/AM_HitHeavy_RP.AM_HitHeavy_RP")))
  (return (LocalVariables|GetDamage%20Animation) (Utilities|Select :Index (Math|Random|RandomIntegerinRange 0 2) :Option%200 "Anim1" :Option%201 "Anim2" :Option%202 "Anim3")))

(fn GetBreachAnimation
  (switch Utilities|FlowControl|Switch|SwitchonE_CharacterPose (Variables|Default|GetCharacter%20Pose)
    (:NewEnumerator1
      (return "LeftPose"))
    (:NewEnumerator2
      (return "RightPose"))))

(fn GetDeathAnimation
  (params (Character%20Pose :type E_CharacterPose%20Enum :default "NewEnumerator1"))
  (switch Utilities|FlowControl|Switch|SwitchonE_CharacterPose Character%20Pose
    (:NewEnumerator1
      (bind _output_get (LocalVariables|SetDeath%20Section (.OutItem (Utilities|Array|Random (Variables|Death|GetDeath%20Montages%20LP)))))
      (switch name _output_get
        (:Variant%201%20LP
          (Variables|Death|SetDeath%20Pose "/Game/Player/Animation/Death/AP_DeathPoseLP_1.AP_DeathPoseLP_1"))
        (:Variant%202%20LP
          (Variables|Death|SetDeath%20Pose "/Game/Player/Animation/Death/AP_DeathPoseLP_2.AP_DeathPoseLP_2"))))
    (:NewEnumerator2
      (bind _output_get_2 (LocalVariables|SetDeath%20Section (.OutItem (Utilities|Array|Random (Variables|Death|GetDeath%20Montages%20RP)))))
      (switch name _output_get_2
        (:Variant%201%20RP
          (Variables|Death|SetDeath%20Pose "/Game/Player/Animation/Death/AP_DeathPoseRP_1.AP_DeathPoseRP_1"))
        (:Variant%202%20RP
          (Variables|Death|SetDeath%20Pose "/Game/Player/Animation/Death/AP_DeathPoseRP_2.AP_DeathPoseRP_2")))))
  (return (LocalVariables|GetDeath%20Section)))

(fn DeathProcessing
  (Components|Animation|SetAnimationMode (Variables|Character|GetMesh) "AnimationSingleNode")
  (Components|Animation|SetAnimation (Variables|Character|GetMesh) (Variables|Death|GetDeath%20Pose))
  (Components|Activation|SetActive (Variables|Character|GetCharacterMovement) false false)
  (Collision|SetCollisionEnabled (Variables|Collision|GetCapsuleComponent) "NoCollision"))

(fn BindEvents
  (EventDispatchers|BindEventtoTakeDamage (Variables|Default|GetAC_Health) (EventDispatchers|CreateEvent :!event Custom|Hit%20Animation))
  (EventDispatchers|BindEventtoIsDead (Variables|Default|GetAC_Health) (EventDispatchers|CreateEvent :!event Custom|Death%20Animation))
  (EventDispatchers|BindEventtoBlockBreached (Variables|Default|GetAC_CombatSystem) (EventDispatchers|CreateEvent :!event Custom|Breach))
  (EventDispatchers|BindEventtoSlowOut (Variables|Default|GetAC_Health) (EventDispatchers|CreateEvent :!event Custom|Damage%20Slow%20Out))
  (EventDispatchers|BindEventtoParryOut (Variables|Default|GetAC_CombatSystem) (EventDispatchers|CreateEvent :!event Custom|Parry%20Out)))

(fn DeathMenuWidget)

(fn ControlWidgetOff)