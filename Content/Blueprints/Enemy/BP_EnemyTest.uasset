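; BP_EnemyTest is a test enemy that starts an assigned behavior tree on its AI controller at BeginPlay.
; On success it seeds the Blackboard with two patrol points, transformed from actor-local to world space, and the player character as the Player key.
; A failed tree start only prints an error; the remaining patrol-point debug prints are never executed.
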(event EventBeginPlay
  (bind _returnvalue (AI|RunBehaviorTree (AI|GetAIController self) (Variables|Default|GetBehaviorTree)))
  (if _returnvalue
    (bind _output_get (Variables|Default|SetBlackboard (AI|GetBlackboard (AI|GetAIController self))))
    (AI|Components|Blackboard|SetValueasVector _output_get (Utilities|Name|MakeLiteralName "PatrolPoint1") (Math|Transform|TransformLocation (Transformation|GetActorTransform) (Variables|Default|GetPatrolPoint1)))
    (AI|Components|Blackboard|SetValueasVector (Variables|Default|GetBlackboard) (Utilities|Name|MakeLiteralName "PatrolPoint2") (Math|Transform|TransformLocation (Transformation|GetActorTransform) (Variables|Default|GetPatrolPoint2)))
    (AI|Components|Blackboard|SetValueasObject (Variables|Default|GetBlackboard) (Utilities|Name|MakeLiteralName "Player") (Game|GetPlayerCharacter 0))
    (else
      (Development|PrintString "Behavior Tree FAILED" true true "(R=1.000000,G=0.000000,B=0.000000,A=1.000000)"))))

(event Collision|EventActorBeginOverlap
  (params (OtherActor :type Actor%20Object%20Reference)))

(event EventTick
  (params (DeltaSeconds :type Float%20%28single-precision%29)))

(fn ConstructionScript)