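; BP_Enemy is an enemy Blueprint driven by an AI controller and its Blackboard.
; On BeginPlay it runs the parent logic, then stores player character 0 under the Blackboard's "Player" key.
; Tick and the construction script are empty, and leftover nodes for printing CharacterState and moving along the right vector are disconnected.
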(event EventBeginPlay
  (|CallParentFunction)
  (bind _output_get (Variables|Default|SetBlackboard (AI|GetBlackboard (AI|GetAIController self))))
  (AI|Components|Blackboard|SetValueasObject _output_get (Utilities|Name|MakeLiteralName "Player") (Game|GetPlayerCharacter 0)))

(event EventTick
  (params (DeltaSeconds :type Float%20%28single-precision%29)))

(fn ConstructionScript)