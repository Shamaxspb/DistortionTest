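; Health component for BP_BaseCharacter that tracks health, healing, full recovery and death.
; TakeDamage derives damage from attack type, boosts it when breached and fires death or hit dispatchers, with debug prints.
; Light attacks also flag the owner as taking damage, halve walk speed and fire SlowOut.
; A separate DamageValidation check rejects dodged or knocked-state hits and hands blocked ones to the combat system component.
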(event EventBeginPlay
  (bind _asbp_base_character (Utilities|Casting|CastToBP_BaseCharacter (Components|GetOwner)))
  (Variables|Default|SetOwner _asbp_base_character))

(fn GetHealth
  (return (Variables|Default|GetHealth)))

(fn GetMaxHealth
  (return (Variables|Default|GetMax%20Health)))

(fn IsDead
  (return (<= (Variables|Default|GetHealth) 0.0)))

(fn Heal
  (params (Amount :type Float%20%28double-precision%29))
  (Variables|Default|SetHealth (Math|Float|Min(Float) (+ (Variables|Default|GetHealth) Amount) (Variables|Default|GetMax%20Health)))
  (Default|CallHealing)
  (return))

(fn Recovery
  (Variables|Default|SetHealth (Variables|Default|GetMax%20Health)))

(fn TakeDamage
  (params (Attack%20Type :type E_AttackType%20Enum :default "NewEnumerator1") (Breached :type Boolean))
  (switch Utilities|FlowControl|Switch|SwitchonE_AttackType Attack%20Type
    (:NewEnumerator1
      (LocalVariables|SetDamage 1e+01)
      (CallFunction|SetDamageVariables)
      (Default|CallSlowOut))
    (:NewEnumerator4
      (LocalVariables|SetDamage 16.5)))
  (if Breached
    (LocalVariables|SetDamage (* (LocalVariables|GetDamage) 1.5)))
  (Variables|Default|SetHealth (Math|Float|Max(Float) (- (Variables|Default|GetHealth) (LocalVariables|GetDamage)) 0.0))
  (if (CallFunction|IsDead)
    (Default|CallIsDead)
    (Development|PrintString "Player died" true true "(R=1.000000,G=0.000000,B=0.000000,A=1.000000)" 3.0)
    (Variables|/Script/Engine.Pawn|SetbUseControllerRotationYaw (Variables|Default|GetOwner) false)
    (else
      (Default|CallTakeDamage Attack%20Type)
      (Development|PrintString (Utilities|String|Append "Target took " (Utilities|String|ToString(Float) (LocalVariables|GetDamage)) " damage") true true "(R=0.760417,G=0.245589,B=0.000000,A=1.000000)" 3.0)
      (Development|PrintString (Utilities|String|Append (Utilities|GetDisplayName (Variables|Default|GetOwner)) " Current HP : " (Utilities|String|ToString(Float) (CallFunction|GetHealth))) true true "(R=0.038204,G=0.610496,B=0.000000,A=1.000000)" 3.0))))

(fn DamageValidation
  (params (Attack%20Type :type E_AttackType%20Enum :default "NewEnumerator1"))
  (if (Utilities|Enum|NotEqual(Enum) (Variables|/Game/Blueprints/BP_BaseCharacter.BP_BaseCharacter_C|GetCharacter%20State (Variables|Default|GetOwner)) "NewEnumerator0")
    (if (Utilities|Enum|NotEqual(Enum) (Variables|/Game/Blueprints/BP_BaseCharacter.BP_BaseCharacter_C|GetCharacter%20State (Variables|Default|GetOwner)) "NewEnumerator3")
      (if (not (Variables|/Game/Blueprints/AC_CombatSystem.AC_CombatSystem_C|GetbKnocked (Variables|/Game/Blueprints/BP_BaseCharacter.BP_BaseCharacter_C|GetAC_CombatSystem (Variables|Default|GetOwner))))
        (return true)
        (else
          (Development|PrintString "Cannot take damage while knocked" true true "(R=0.760417,G=0.245589,B=0.000000,A=1.000000)" 3.0)
          (return false)))
      (else
        (Default|TakeHitinBlock (Variables|/Game/Blueprints/BP_BaseCharacter.BP_BaseCharacter_C|GetAC_CombatSystem (Variables|Default|GetOwner)) Attack%20Type)
        (return false)))
    (else
      (Development|PrintString "Damage Dodged" true true "(R=0.760417,G=0.245589,B=0.000000,A=1.000000)" 3.0)
      (return false))))

(fn SetDamageVariables
  (bind _owner (Variables|Default|GetOwner))
  (Variables|/Game/Blueprints/BP_BaseCharacter.BP_BaseCharacter_C|SetbTakingDamage (Variables|Default|GetOwner) true)
  (Variables|/Script/Engine.CharacterMovementComponent|SetMaxWalkSpeed (Variables|/Script/Engine.Character|GetCharacterMovement _owner) (* (Variables|/Game/Blueprints/AC_CombatSystem.AC_CombatSystem_C|GetDefault%20Move%20Speed (Variables|/Game/Blueprints/BP_BaseCharacter.BP_BaseCharacter_C|GetAC_CombatSystem _owner)) 0.5)))