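; Player health component that tracks health with damage, healing, full recovery and death checks.
; It caches the BP_Player character on BeginPlay and plays montages on its mesh.
; Non-lethal damage plays a random section of a light or heavy hit montage chosen by attack type.
; Lethal damage plays a random death montage section and disables the player's controller yaw rotation.
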(event Custom|Hit%20Reaction
  (params (MontageToPlay :type Anim%20Montage%20Object%20Reference) (StartingSection :type Name))
  (Animation|Montage|PlayMontage (Variables|/Script/Engine.Character|GetMesh (Variables|Default|GetPlayer)) MontageToPlay 1.25 0.0 StartingSection))

(event Custom|Death%20Animation
  (bind _player (Variables|Default|GetPlayer))
  (Animation|Montage|PlayMontage (Variables|/Script/Engine.Character|GetMesh _player) "/Game/Player/Animation/Death/AM_Death.AM_Death" 1.0 0.0 (.OutItem (Utilities|Array|Random (Variables|/Game/Blueprints/BP_Player.BP_Player_C|GetDeath%20Montages _player)))))

(event EventBeginPlay
  (bind _asbp_player (Utilities|Casting|CastToBP_Player (Game|GetPlayerCharacter 0)))
  (Variables|Default|SetPlayer _asbp_player))

(fn GetHealth
  (return (Variables|Default|GetHealth)))

(fn IsDead
  (return (<= (Variables|Default|GetHealth) 0.0)))

(fn Heal
  (params (Amount :type Float%20%28double-precision%29))
  (Variables|Default|SetHealth (Math|Float|Min(Float) (+ (Variables|Default|GetHealth) Amount) (Variables|Default|GetMax%20Health))))

(fn Recovery
  (Variables|Default|SetHealth (Variables|Default|GetMax%20Health)))

(fn TakeDamage
  (params (Damage :type Float%20%28double-precision%29) (Attack%20Type :type E_AttackType%20Enum :default "NewEnumerator1"))
  (Variables|Default|SetHealth (Math|Float|Max(Float) (- (Variables|Default|GetHealth) Damage) 0.0))
  (if (CallFunction|IsDead)
    (CallFunction|DeathAnimation)
    (Development|PrintString "Player died" true true "(R=1.000000,G=0.000000,B=0.000000,A=1.000000)" 3.0)
    (Variables|/Script/Engine.Pawn|SetbUseControllerRotationYaw (Variables|Default|GetPlayer) false)
    (return Damage)
    (else
      (bind (_montage _section) (CallFunction|GetTakeDamageAnimation Attack%20Type))
      (CallFunction|HitReaction _montage _section)
      (Development|PrintString (Utilities|String|Append "Player took " (Utilities|String|ToString(Float) Damage) " damage") true true "(R=0.760417,G=0.245589,B=0.000000,A=1.000000)" 3.0)
      (return Damage))))

(fn GetTakeDamageAnimation
  (params (Attack%20Type :type E_AttackType%20Enum :default "NewEnumerator1"))
  (switch Utilities|FlowControl|Switch|SwitchonE_AttackType Attack%20Type
    (:NewEnumerator1
      (return "/Game/Player/Animation/TakeDamage/AM_HitLight.AM_HitLight" (Utilities|Select :Index (Math|Random|RandomIntegerinRange 0 1) :Option%200 "Anim1" :Option%201 "Anim2")))
    (:NewEnumerator4
      (return "/Game/Player/Animation/TakeDamage/AM_HitHeavy.AM_HitHeavy" (Utilities|Select :Index (Math|Random|RandomIntegerinRange 0 2) :Option%200 "Anim1" :Option%201 "Anim2" :Option%202 "Anim3")))))