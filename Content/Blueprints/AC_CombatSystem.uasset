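; Actor component on BP_BaseCharacter owners that runs spear melee combat: directional light and heavy combos, dodging and blocking.
; Validators gate actions on character state, and attack counters select montage sections for combo hits.
; Timer-driven sphere traces along spear sockets damage each character once per swing through ACHealth.
; Blocked hits build a decaying Breach meter that, when full, breaks the guard, disarming and knocking the owner.
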(event Input|EnhancedActionEvents|EnhancedInputActionIA_LightAttack
  (params (ActionValue :type Boolean) (ElapsedSeconds :type Float%20%28double-precision%29) (TriggeredSeconds :type Float%20%28double-precision%29) (InputAction :type Input%20Action%20Object%20Reference :default "/Game/Player/Input/Actions/IA_LightAttack.IA_LightAttack"))
  ;[0.7157 0.1384 0.09306] Attack
  (:Started
    (Variables|Default|SetInput%20Action InputAction)
    (CallFunction|LightAttack)))

(event Input|EnhancedActionEvents|EnhancedInputActionIA_Block
  (params (ActionValue :type Boolean) (ElapsedSeconds :type Float%20%28double-precision%29) (TriggeredSeconds :type Float%20%28double-precision%29) (InputAction :type Input%20Action%20Object%20Reference :default "/Game/Player/Input/Actions/IA_Block.IA_Block"))
  ;[1 0.2462 0] Block
  (:Started
    (CallFunction|BlockStart))
  (:Completed
    (CallFunction|BlockStop)))

(event Input|EnhancedActionEvents|EnhancedInputActionIA_Dodge
  (params (ActionValue :type Vector%202D%20Structure) (ElapsedSeconds :type Float%20%28double-precision%29) (TriggeredSeconds :type Float%20%28double-precision%29) (InputAction :type Input%20Action%20Object%20Reference :default "/Game/Player/Input/Actions/IA_Dodge.IA_Dodge"))
  ;[1 0.2023 0.7443] Dodge
  (:Started
    (CallFunction|Dodge)))

(event Input|EnhancedActionEvents|EnhancedInputActionIA_HeavyAttack
  (params (ActionValue :type Boolean) (ElapsedSeconds :type Float%20%28double-precision%29) (TriggeredSeconds :type Float%20%28double-precision%29) (InputAction :type Input%20Action%20Object%20Reference :default "/Game/Player/Input/Actions/IA_HeavyAttack.IA_HeavyAttack"))
  ;[0.7157 0.1384 0.09306] Attack
  (:Started
    (Variables|Default|SetInput%20Action InputAction)
    (CallFunction|HeavyAttack)))

(event EventBeginPlay
  (bind _asbp_base_character (Utilities|Casting|CastToBP_BaseCharacter (Components|GetOwner)))
  (Variables|Default|SetOwner _asbp_base_character)
  (bind _asbp_player (Utilities|Casting|CastToBP_Player (Components|GetOwner)))
  (Variables|Default|SetPlayer _asbp_player))

(event Custom|Dodge%20Enemy
  (if (and (Utilities|Enum|NotEqual(Enum) (Variables|/Game/Blueprints/BP_BaseCharacter.BP_BaseCharacter_C|GetCharacter%20State (Variables|Default|GetOwner)) "NewEnumerator0") (Variables|Dodge|GetbCanDodge))
    (if (not (Variables|/Game/Blueprints/BP_BaseCharacter.BP_BaseCharacter_C|GetbTakingDamage (Variables|Default|GetOwner)))
      (Variables|/Game/Blueprints/BP_BaseCharacter.BP_BaseCharacter_C|SetCharacter%20State (Variables|Default|GetOwner) "NewEnumerator0")
      (Animation|Montage|PlayMontage (Variables|/Script/Engine.Character|GetMesh (Variables|Default|GetOwner)) "/Game/Player/Animation/Dodge/AM_DodgeLP.AM_DodgeLP" 1.0 0.0 (.OutItem (Utilities|Array|Random (Utilities|Array|MakeArray "Backward" "Right" "Left")))
        (:OnBlendOut
          (Variables|/Game/Blueprints/BP_BaseCharacter.BP_BaseCharacter_C|SetCharacter%20State (Variables|Default|GetOwner) "NewEnumerator1")
          (Default|CallDodgeEnd)))
      (else
        (Development|PrintString "Enemy: Cannot Dodge while taking damage" true true "(R=1.000000,G=0.000000,B=0.000000,A=1.000000)")))
    (else
      (Development|PrintString "Enemy: Dodge is in process" true true "(R=1.000000,G=0.000000,B=0.000000,A=1.000000)"))))

(event Custom|Dodge
  (if (and (Utilities|Enum|NotEqual(Enum) (Variables|/Game/Blueprints/BP_BaseCharacter.BP_BaseCharacter_C|GetCharacter%20State (Variables|Default|GetPlayer)) "NewEnumerator0") (Variables|Dodge|GetbCanDodge))
    (if (not (Variables|/Game/Blueprints/BP_BaseCharacter.BP_BaseCharacter_C|GetbTakingDamage (Variables|Default|GetPlayer)))
      (Variables|Attack|SetLight%20Attack%20Count 0)
      (Variables|Attack|SetHeavy%20Attack%20Count 0)
      (Variables|Dodge|SetbCanDodge false)
      (Variables|/Game/Blueprints/BP_BaseCharacter.BP_BaseCharacter_C|SetCharacter%20State (Variables|Default|GetPlayer) "NewEnumerator0")
      (Variables|/Script/Engine.Pawn|SetbUseControllerRotationYaw (Variables|Default|GetPlayer) false)
      (bind (_dodge_montage _dodge_direction) (Dodge|FindDodgeAnimation))
      (Animation|Montage|PlayMontage (Variables|/Script/Engine.Character|GetMesh (Variables|Default|GetPlayer)) _dodge_montage 1.0 0.0 _dodge_direction
        (:OnBlendOut
          (Variables|/Game/Blueprints/BP_BaseCharacter.BP_BaseCharacter_C|SetCharacter%20State (Variables|Default|GetPlayer) "NewEnumerator1")
          (Default|RotatetoCamera (Variables|Default|GetPlayer))))
      (else
        (Development|PrintString "Cannot Dodge while taking damage" true true "(R=1.000000,G=0.000000,B=0.000000,A=1.000000)")))
    (else
      (Development|PrintString "Dodge is in process" true true "(R=1.000000,G=0.000000,B=0.000000,A=1.000000)"))))

(event Custom|Start%20Breach%20Decreasing
  ;[1 0.2107 0.07292] Breach
  (bind _returnvalue (Utilities|Time|SetTimerbyEvent (delegate Custom|Breach%20Decreasing) 0.05 true))
  (Variables|Block|SetBreach%20Decrease%20Timer _returnvalue)
  (Development|PrintString "Breach Decreasing: Started" true true "(R=1.000000,G=1.000000,B=0.000000,A=1.000000)" 3.0))

(event Custom|Block%20Slow%20Out
  (Variables|/Script/Engine.CharacterMovementComponent|SetMaxWalkSpeed (Variables|/Script/Engine.Character|GetCharacterMovement (Variables|Default|GetOwner)) (Variables|Block|GetDefault%20Move%20Speed)))

(event Custom|Block%20Slow%20In
  (Variables|/Script/Engine.CharacterMovementComponent|SetMaxWalkSpeed (Variables|/Script/Engine.Character|GetCharacterMovement (Variables|Default|GetOwner)) (Variables|Block|GetBlock%20Move%20Speed)))

(event Custom|Block%20Stop
  ;[1 0.376 0.07292] Block
  (if (Utilities|Enum|Equal(Enum) (Variables|/Game/Blueprints/BP_BaseCharacter.BP_BaseCharacter_C|GetCharacter%20State (Variables|Default|GetOwner)) "NewEnumerator3")
    (Variables|/Game/Blueprints/BP_BaseCharacter.BP_BaseCharacter_C|SetCharacter%20State (Variables|Default|GetOwner) "NewEnumerator1")
    (Animation|StopAnimMontage (Variables|Default|GetOwner) 0)
    (CallFunction|BlockSlowOut)))

(event Custom|Block%20Start
  ;[1 0.376 0.07292] Block
  (bind _can_block (Block|BlockValidation))
  (if _can_block
    (Variables|/Game/Blueprints/BP_BaseCharacter.BP_BaseCharacter_C|SetCharacter%20State (Variables|Default|GetOwner) "NewEnumerator3")
    (Animation|StopAnimMontage (Variables|Default|GetOwner) 0)
    (CallFunction|BlockSlowin)))

(event Custom|Breach%20Decreasing
  ;[1 0.2107 0.07292] Breach
  (if (> (Variables|Block|GetCurrent%20Breach) 0.0)
    (Math|Float|DecrementFloat (Variables|Block|GetCurrent%20Breach))
    (else
      (Utilities|Time|ClearandInvalidateTimerbyHandle (Variables|Block|GetBreach%20Decrease%20Timer))
      (Variables|Block|SetbDisarmed false)
      (Development|PrintString "Breach Decreasing: Finished" true true "(R=0.760417,G=0.245589,B=0.000000,A=1.000000)" 3.0))))

(event Custom|Attack%20Left
  ;[0.7157 0.1384 0.09306] Attack
  (Animation|Montage|PlayMontage (Variables|/Script/Engine.Character|GetMesh (Variables|Default|GetOwner)) "/Game/Player/Animation/Attack/AM_LightAttackLP_Directional.AM_LightAttackLP_Directional" 1.25 0.0 "Left"
    (:OnBlendOut
      (Variables|/Game/Blueprints/BP_BaseCharacter.BP_BaseCharacter_C|SetCharacter%20State (Variables|Default|GetOwner) "NewEnumerator1"))
    (:OnInterrupted
      (Variables|Attack|SetbContinueCombo false))))

(event Custom|Stop%20Spear%20Trace
  ;[1 0.1354 0.2239] Damage Processing
  (Utilities|Map|Clear (Variables|Attack|GetHit%20Characters))
  (Utilities|Time|ClearandInvalidateTimerbyHandle (Variables|Attack|GetSpear%20Trace%20Timer)))

(event Custom|Light%20Attack%20Place
  ;[0.7157 0.1384 0.09306] Attack
  (Animation|Montage|PlayMontage (Variables|/Script/Engine.Character|GetMesh (Variables|Default|GetOwner)) "/Game/Player/Animation/Attack/AM_LightAttackLP_Place.AM_LightAttackLP_Place" 1.25 0.0 (Attack|GetAttackSequence "NewEnumerator1")
    (:then
      (Math|Integer|IncrementInt (Variables|Attack|GetLight%20Attack%20Count)))))

(event Custom|Light%20Attack%20Forward
  ;[0.7157 0.1384 0.09306] Attack
  (Animation|Montage|PlayMontage (Variables|/Script/Engine.Character|GetMesh (Variables|Default|GetOwner)) "/Game/Player/Animation/Attack/AM_LightAttackLP_Forward.AM_LightAttackLP_Forward" 1.25 0.0 (Attack|GetAttackSequence "NewEnumerator1")
    (:then
      (Math|Integer|IncrementInt (Variables|Attack|GetLight%20Attack%20Count)))))

(event Custom|Spear%20Hit
  (bind _owner (Variables|Default|GetOwner))
  (bind _sm_spear (Variables|/Game/Blueprints/BP_BaseCharacter.BP_BaseCharacter_C|GetSM_Spear _owner))
  ;[1 0.1354 0.2239] Damage Processing
  (bind (_outhits _returnvalue) (Collision|MultiSphereTraceByChannel (Transformation|GetSocketLocation _sm_spear "Top") (Transformation|GetSocketLocation _sm_spear "Bottom") 7.5 "TraceTypeQuery1" false 0 "ForDuration"))
  (if _returnvalue
    (for _array_element _outhits
      (bind _asbp_base_character (Utilities|Casting|CastToBP_BaseCharacter (.HitActor (Collision|BreakHitResult _array_element))))
      (bind _output_get (Variables|Attack|SetHit%20Character _asbp_base_character))
      (if (not (.ReturnValue (Utilities|Map|Find (Variables|Attack|GetHit%20Characters) _output_get)))
        (Utilities|Map|Add (Variables|Attack|GetHit%20Characters) (Variables|Attack|GetHit%20Character) 0)
        (bind _can_take_damage (Default|DamageValidation (Variables|/Game/Blueprints/BP_BaseCharacter.BP_BaseCharacter_C|GetAC_Health (Variables|Attack|GetHit%20Character)) (Variables|Attack|GetAttack%20Type)))
        (if _can_take_damage
          (Default|TakeDamage (Variables|/Game/Blueprints/BP_BaseCharacter.BP_BaseCharacter_C|GetAC_Health (Variables|Attack|GetHit%20Character)) (Variables|Attack|GetAttack%20Type) false))))))

(event Custom|Heavy%20Attack
  ;[0.7157 0.1384 0.09306] Attack
  (bind _can_attack (Attack|AttackValidation))
  (if _can_attack
    (Variables|/Game/Blueprints/BP_BaseCharacter.BP_BaseCharacter_C|SetCharacter%20State (Variables|Default|GetOwner) "NewEnumerator4")
    (Variables|Attack|SetAttack%20Type "NewEnumerator4")
    (switch Utilities|FlowControl|Switch|SwitchonE_DodgeDirection (Variables|/Game/Blueprints/BP_Player.BP_Player_C|GetDodge%20Direction (Variables|Default|GetPlayer))
      (:NewEnumerator0
        (bind _do_next_hit (Attack|HeavyComboValidator 2))
        (if _do_next_hit
          (CallFunction|HeavyAttackForward)
          (Variables|Attack|SetbContinueCombo false :!label _label)))
      (:NewEnumerator1
        (Variables|/Game/Blueprints/BP_BaseCharacter.BP_BaseCharacter_C|SetCharacter%20State (Variables|Default|GetOwner) "NewEnumerator1" :!label _label_2)
        (goto _label))
      (:NewEnumerator2
        (goto _label_2))
      (:NewEnumerator3
        (goto _label_2))
      (:NewEnumerator5
        (bind _do_next_hit_2 (Attack|HeavyComboValidator 3))
        (if _do_next_hit_2
          (CallFunction|HeavyAttackPlace)
          (goto _label))))))

(event Custom|Knockback%20Attack)

(event Custom|Heavy%20Attack%20Forward
  ;[0.7157 0.1384 0.09306] Attack
  (Animation|Montage|PlayMontage (Variables|/Script/Engine.Character|GetMesh (Variables|Default|GetOwner)) "/Game/Player/Animation/Attack/AM_HeavyAttackLP_Forward.AM_HeavyAttackLP_Forward" 1.0 0.0 (Attack|GetAttackSequence "NewEnumerator4")
    (:then
      (Math|Integer|IncrementInt (Variables|Attack|GetHeavy%20Attack%20Count)))))

(event Custom|Heavy%20Attack%20Place
  ;[0.7157 0.1384 0.09306] Attack
  (Animation|Montage|PlayMontage (Variables|/Script/Engine.Character|GetMesh (Variables|Default|GetOwner)) "/Game/Player/Animation/Attack/AM_HeavyAttackLP_Place.AM_HeavyAttackLP_Place" 1.0 0.0 (Attack|GetAttackSequence "NewEnumerator4")
    (:then
      (Math|Integer|IncrementInt (Variables|Attack|GetHeavy%20Attack%20Count)))))

(event Custom|Light%20Attack
  ;[0.7157 0.1384 0.09306] Attack
  (bind _can_attack (Attack|AttackValidation))
  (if _can_attack
    (Variables|/Game/Blueprints/BP_BaseCharacter.BP_BaseCharacter_C|SetCharacter%20State (Variables|Default|GetOwner) "NewEnumerator4")
    (Variables|Attack|SetAttack%20Type "NewEnumerator1")
    (switch Utilities|FlowControl|Switch|SwitchonE_AttackDirection (Variables|/Game/Blueprints/BP_Player.BP_Player_C|GetAttack%20Direction (Variables|Default|GetPlayer))
      (:NewEnumerator0
        (bind _do_next_hit (Attack|LightComboValidator 5))
        (if _do_next_hit
          (CallFunction|LightAttackForward)
          (Variables|Attack|SetbContinueCombo false :!label _label)))
      (:NewEnumerator1
        (CallFunction|AttackBackward)
        (goto _label))
      (:NewEnumerator2
        (CallFunction|AttackRight)
        (goto _label))
      (:NewEnumerator3
        (CallFunction|AttackLeft)
        (goto _label))
      (:NewEnumerator5
        (bind _do_next_hit_2 (Attack|LightComboValidator 4))
        (if _do_next_hit_2
          (CallFunction|LightAttackPlace)
          (goto _label))))))

(event Custom|Start%20Spear%20Trace
  ;[1 0.1354 0.2239] Damage Processing
  (bind _returnvalue (Utilities|Time|SetTimerbyEvent (delegate Custom|Spear%20Hit) 0.01 true))
  (Variables|Attack|SetSpear%20Trace%20Timer _returnvalue))

(event Custom|Attack%20Backward
  ;[0.7157 0.1384 0.09306] Attack
  (Animation|Montage|PlayMontage (Variables|/Script/Engine.Character|GetMesh (Variables|Default|GetOwner)) "/Game/Player/Animation/Attack/AM_LightAttackLP_Directional.AM_LightAttackLP_Directional" 1.25 0.0 "Backward"
    (:OnBlendOut
      (Variables|/Game/Blueprints/BP_BaseCharacter.BP_BaseCharacter_C|SetCharacter%20State (Variables|Default|GetOwner) "NewEnumerator1"))
    (:OnInterrupted
      (Variables|Attack|SetbContinueCombo false))))

(event Custom|Attack%20Right
  ;[0.7157 0.1384 0.09306] Attack
  (Animation|Montage|PlayMontage (Variables|/Script/Engine.Character|GetMesh (Variables|Default|GetOwner)) "/Game/Player/Animation/Attack/AM_LightAttackLP_Directional.AM_LightAttackLP_Directional" 1.25 0.0 "Right"
    (:OnBlendOut
      (Variables|/Game/Blueprints/BP_BaseCharacter.BP_BaseCharacter_C|SetCharacter%20State (Variables|Default|GetOwner) "NewEnumerator1"))
    (:OnInterrupted
      (Variables|Attack|SetbContinueCombo false))))

(fn FindDodgeAnimation
  (bind _player (Variables|Default|GetPlayer))
  (bind _dodge_animation_section (Variables|Dodge|GetDodge%20Animation%20Section))
  (bind _dodge_direction (Variables|/Game/Blueprints/BP_Player.BP_Player_C|GetDodge%20Direction _player))
  (bind _value (Utilities|Map|Find _dodge_animation_section _dodge_direction))
  (switch Utilities|FlowControl|Switch|SwitchonE_CharacterPose (Variables|/Game/Blueprints/BP_BaseCharacter.BP_BaseCharacter_C|GetCharacter%20Pose (Variables|Default|GetOwner))
    (:NewEnumerator1
      (return "/Game/Player/Animation/Dodge/AM_DodgeLP.AM_DodgeLP" _value))
    (:NewEnumerator2
      (return "/Game/Player/Animation/Dodge/AM_DodgeRP.AM_DodgeRP" _value))))

(fn AttackValidation
  (if (Utilities|Enum|NotEqual(Enum) (Variables|/Game/Blueprints/BP_BaseCharacter.BP_BaseCharacter_C|GetCharacter%20State (Variables|Default|GetOwner)) "NewEnumerator0")
    (if (Utilities|Enum|NotEqual(Enum) (Variables|/Game/Blueprints/BP_BaseCharacter.BP_BaseCharacter_C|GetCharacter%20State (Variables|Default|GetOwner)) "NewEnumerator3")
      (if (not (Variables|Block|GetbKnocked))
        (if (Utilities|Enum|NotEqual(Enum) (Variables|/Game/Blueprints/BP_BaseCharacter.BP_BaseCharacter_C|GetCharacter%20State (Variables|Default|GetOwner)) "NewEnumerator4")
          (return true)
          (elif (Variables|Attack|GetbComboWindowOpened)
            (Variables|Attack|SetbContinueCombo true)
            (return false)
            (else
              (Development|PrintString "Attack is in process" true true "(R=1.000000,G=0.000000,B=0.000000,A=1.000000)" 1.0)
              (return false))))
        (else
          (Development|PrintString "Cannot attack during Knockdown" true true "(R=1.000000,G=0.000000,B=0.000000,A=1.000000)" 1.0)
          (return false)))
      (else
        (Development|PrintString "Knockback Attack" true true "(R=0.760417,G=0.245589,B=0.000000,A=1.000000)" 1.0)
        (CallFunction|KnockbackAttack)
        (return false)))
    (else
      (Development|PrintString "Cannot attack during Dodge" true true "(R=1.000000,G=0.000000,B=0.000000,A=1.000000)" 1.0)
      (return false))))

(fn LightComboValidator
  (params (Max%20Combo%20Counter :type Integer))
  (if (< (Variables|Attack|GetLight%20Attack%20Count) Max%20Combo%20Counter)
    (return true)
    (else
      (Development|PrintString "Combo attack limit reached" true true "(R=0.760417,G=0.245589,B=0.000000,A=1.000000)" 3.0)
      (Variables|/Game/Blueprints/BP_BaseCharacter.BP_BaseCharacter_C|SetCharacter%20State (Variables|Default|GetPlayer) "NewEnumerator1")
      (Variables|Attack|SetbContinueCombo false)
      (Variables|Attack|SetLight%20Attack%20Count 0)
      (return false))))

(fn HeavyComboValidator
  (params (Max%20Combo%20Counter :type Integer))
  (if (< (Variables|Attack|GetHeavy%20Attack%20Count) Max%20Combo%20Counter)
    (return true)
    (else
      (Development|PrintString "Combo attack limit reached" true true "(R=0.760417,G=0.245589,B=0.000000,A=1.000000)" 3.0)
      (Variables|/Game/Blueprints/BP_BaseCharacter.BP_BaseCharacter_C|SetCharacter%20State (Variables|Default|GetPlayer) "NewEnumerator1")
      (Variables|Attack|SetbContinueCombo false)
      (Variables|Attack|SetHeavy%20Attack%20Count 0)
      (return false))))

(fn GetAttackSequence
  (params (Attack%20Type :type E_AttackType%20Enum :default "NewEnumerator1"))
  (switch Utilities|FlowControl|Switch|SwitchonE_AttackType Attack%20Type
    (:NewEnumerator1
      (LocalVariables|SetAttack%20Count (Variables|Attack|GetLight%20Attack%20Count)))
    (:NewEnumerator4
      (LocalVariables|SetAttack%20Count (Variables|Attack|GetHeavy%20Attack%20Count))))
  (return (Utilities|Select :Index (LocalVariables|GetAttack%20Count) :Option%200 "1st Hit" :Option%201 "2nd Hit" :Option%202 "3rd Hit" :Option%203 "4th Hit" :Option%204 "5th Hit" :Option%205 "6th Hit")))

(fn GetBreach
  (return (Variables|Block|GetCurrent%20Breach)))

(fn GetMaxBreach
  (return (Variables|Block|GetMax%20Breach)))

(fn TakeHitinBlock
  (params (Attack%20Type :type E_AttackType%20Enum :default "NewEnumerator1"))
  (bind _owner (Variables|Default|GetOwner))
  (bind _charactermovement (Variables|/Script/Engine.Character|GetCharacterMovement _owner))
  (LocalVariables|SetTakenHit Attack%20Type)
  (Variables|/Game/Blueprints/BP_BaseCharacter.BP_BaseCharacter_C|SetBlock%20Impact (Variables|Default|GetOwner) true)
  (Variables|/Game/Blueprints/BP_BaseCharacter.BP_BaseCharacter_C|SetPrevious%20Move%20Speed _owner (Variables|/Script/Engine.CharacterMovementComponent|GetMaxWalkSpeed _charactermovement))
  (Variables|/Script/Engine.CharacterMovementComponent|SetMaxWalkSpeed _charactermovement (* (Variables|/Script/Engine.CharacterMovementComponent|GetMaxWalkSpeed _charactermovement) 0.5))
  (switch Utilities|FlowControl|Switch|SwitchonE_AttackType (LocalVariables|GetTakenHit)
    (:NewEnumerator1
      (Variables|Block|SetCurrent%20Breach (+ (Variables|Block|GetCurrent%20Breach) (Variables|Block|GetBreach%20Light%20Increase))))
    (:NewEnumerator4
      (Variables|Block|SetCurrent%20Breach (+ (Variables|Block|GetCurrent%20Breach) (Variables|Block|GetBreach%20Heavy%20Increase)))))
  (Development|PrintString (Utilities|String|Append (Utilities|GetDisplayName (Variables|Default|GetOwner)) " took " (Utilities|String|EnumtoString (LocalVariables|GetTakenHit))) true true "(R=0.760417,G=0.245589,B=0.000000,A=1.000000)")
  (if (>= (Variables|Block|GetCurrent%20Breach) (Variables|Block|GetMax%20Breach))
    (Block|BreachBlock (LocalVariables|GetTakenHit))
    (else
      (Development|PrintString "Damage Blocked" true true "(R=0.760417,G=0.245589,B=0.000000,A=1.000000)" 3.0)
      (CallFunction|StartBreachDecreasing))))

(fn BlockValidation
  (if (Utilities|Enum|NotEqual(Enum) (Variables|/Game/Blueprints/BP_BaseCharacter.BP_BaseCharacter_C|GetCharacter%20State (Variables|Default|GetOwner)) "NewEnumerator0")
    (if (not (Variables|Block|GetbDisarmed))
      (Variables|Attack|SetLight%20Attack%20Count 0)
      (Variables|Attack|SetHeavy%20Attack%20Count 0)
      (return true)
      (else
        (Development|PrintString "Cannot block while Disarmed" true true "(R=1.000000,G=0.000000,B=0.000000,A=1.000000)")))
    (else
      (Development|PrintString "Cannot block during Dodge" true true "(R=1.000000,G=0.000000,B=0.000000,A=1.000000)")))
  (return false))

(fn BreachBlock
  (params (Taken%20Hit :type E_AttackType%20Enum :default "NewEnumerator1"))
  (Variables|Block|SetCurrent%20Breach (Math|Float|Min(Float) (Variables|Block|GetMax%20Breach) (Variables|Block|GetCurrent%20Breach)))
  (Development|PrintString "Block Breached" true true "(R=1.000000,G=0.000000,B=0.000000,A=1.000000)" 3.0)
  (Variables|Block|SetbDisarmed true)
  (Variables|Block|SetbKnocked true)
  (Variables|/Script/Engine.Pawn|SetbUseControllerRotationYaw (Variables|Default|GetOwner) false)
  (Variables|/Game/Blueprints/BP_BaseCharacter.BP_BaseCharacter_C|SetCharacter%20State (Variables|Default|GetOwner) "NewEnumerator1")
  (Default|TakeDamage (Variables|/Game/Blueprints/BP_BaseCharacter.BP_BaseCharacter_C|GetAC_Health (Variables|Default|GetOwner)) Taken%20Hit true)
  (Default|CallBlockBreached))